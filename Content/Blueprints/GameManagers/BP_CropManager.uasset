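; BP_CropManager is an actor that turns spoken farm commands into a numeric selection.
; On BeginPlay it binds TriggerSpeech to the speech recognition subsystem's words-spoken event.
; TriggerSpeech checks each recognized phrase against "farm one" through "farm five" in a nested branch chain and stores the zero-based index in Count.
; Count is printed for debugging on all but the last match, and nothing here uses it further.
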(event Custom|TriggerSpeech
  (params (Text :type Recognised%20Phrases%20Structure))
  (for _array_element (Utilities|Struct|BreakRecognisedPhrases Text)
    (if (Utilities|Enum|Equal(Enum) _array_element "farm one")
      (bind _output_get (Variables|Default|Setcount 0))
      (Development|PrintString (Utilities|String|ToString(Integer) _output_get))
      (elif (Utilities|Enum|Equal(Enum) _array_element "farm two")
        (bind _output_get_2 (Variables|Default|Setcount 1))
        (Development|PrintString (Utilities|String|ToString(Integer) _output_get_2))
        (elif (Utilities|Enum|Equal(Enum) _array_element "farm three")
          (bind _output_get_3 (Variables|Default|Setcount 2))
          (Development|PrintString (Utilities|String|ToString(Integer) _output_get_3))
          (elif (Utilities|Enum|Equal(Enum) _array_element "farm four")
            (bind _output_get_4 (Variables|Default|Setcount 3))
            (Development|PrintString (Utilities|String|ToString(Integer) _output_get_4))
            (elif (Utilities|Enum|Equal(Enum) _array_element "farm five")
              (Variables|Default|Setcount 4))))))))

(event EventBeginPlay
  (EventDispatchers|BindEventtoOnWordsSpoken (Subsystems|GetSpeechRecognitionSubsystem) (delegate Custom|TriggerSpeech)))

(event Collision|EventActorBeginOverlap
  (params (OtherActor :type Actor%20Object%20Reference)))

(event EventTick
  (params (DeltaSeconds :type Float%20%28single-precision%29)))

(fn ConstructionScript)