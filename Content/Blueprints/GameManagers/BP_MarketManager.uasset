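; BP_MarketManager is a game manager that opens the market screen by voice command.
; On BeginPlay it binds TriggerSpeech to the speech recognition subsystem's words-spoken event.
; When a recognized phrase is "open market", it removes all widgets, adds a WBP_CropsInfo widget to the viewport and shows the mouse cursor.
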(event Custom|TriggerSpeech
  (params (Text :type Recognised%20Phrases%20Structure))
  (for _array_element (Utilities|Struct|BreakRecognisedPhrases Text)
    (if (Utilities|Enum|Equal(Enum) _array_element "open market")
      (Viewport|RemoveAllWidgets)
      (bind _returnvalue (UserInterface|CreateWidget "/Game/Widgets/WBP_CropsInfo.WBP_CropsInfo_C"))
      (UserInterface|Viewport|AddtoViewport _returnvalue 0)
      (Variables|/Script/Engine.PlayerController|SetbShowMouseCursor (Game|GetPlayerController 0) true))))

(event EventBeginPlay
  (EventDispatchers|BindEventtoOnWordsSpoken (Subsystems|GetSpeechRecognitionSubsystem) (delegate Custom|TriggerSpeech)))

(event EventTick
  (params (DeltaSeconds :type Float%20%28single-precision%29)))

(fn ConstructionScript)