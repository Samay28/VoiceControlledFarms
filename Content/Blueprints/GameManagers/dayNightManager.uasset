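; Day/night manager that rotates itself in pitch over time and switches fire and lantern lights to match.
; BeginPlay adds the main game HUD widget and caches all BP_Fire and BP_Lantern actors.
; Every Tick sets fire particle and light visibility by whether pitch is within a fixed window.
; The lantern loop is nested inside the fire loop, so lanterns update once per fire, never without one.
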(event EventBeginPlay
  (bind _returnvalue (UserInterface|CreateWidget "/Game/Widgets/WBP_MainGame.WBP_MainGame_C"))
  (UserInterface|Viewport|AddtoViewport _returnvalue 0)
  (bind _outactors (Actor|GetAllActorsOfClass "/Game/Blueprints/BP_Lantern.BP_Lantern_C"))
  (bind _outactors_2 (Actor|GetAllActorsOfClass "/Game/Blueprints/BP_Fire.BP_Fire_C"))
  (Variables|Default|SetFireLightArray _outactors_2)
  (Variables|Default|SetLanternArray _outactors))

(event EventTick
  (params (DeltaSeconds :type Float%20%28single-precision%29))
  (bind _returnvalue (Transformation|GetActorRotation))
  (Transformation|AddActorLocalRotation (Math|Rotator|MakeRotator 0.0 (* DeltaSeconds (Variables|Default|GetSpeed)) 0.0) false false)
  (if (and (> (.pitch _returnvalue) -15.0) (< (.pitch _returnvalue) 91.0))
    (for _array_element (Variables|Default|GetFireLightArray)
      (Rendering|SetVisibility (Variables|/Game/Blueprints/BP_Fire.BP_Fire_C|GetMeshes_Particles_Fire_01 _array_element) true false)
      (for _array_element_2 (Variables|Default|GetLanternArray)
        (Rendering|SetVisibility (Variables|/Game/Blueprints/BP_Lantern.BP_Lantern_C|GetPointLight _array_element_2) true false)))
    (elif true
      (for _array_element_3 (Variables|Default|GetFireLightArray)
        (Rendering|SetVisibility (Variables|/Game/Blueprints/BP_Fire.BP_Fire_C|GetMeshes_Particles_Fire_01 _array_element_3) false false)
        (for _array_element_4 (Variables|Default|GetLanternArray)
          (Rendering|SetVisibility (Variables|/Game/Blueprints/BP_Lantern.BP_Lantern_C|GetPointLight _array_element_4) false false))))))

(fn ConstructionScript)