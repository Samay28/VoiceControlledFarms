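; BP_UtilCommand is a voice command handler that opens a utility farm widget when the player says "cutting".
; On BeginPlay it binds to the speech recognition subsystem's words-spoken event and checks each recognized phrase for that keyword.
; On a match it reads Count from BP_CropManager and adds one of five WBP_UtilityFarm widgets to the viewport, chosen through nested branches on that value.
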(event Custom|TriggerSpeech
  (params (Text :type Recognised%20Phrases%20Structure))
  (for _array_element (Utilities|Struct|BreakRecognisedPhrases Text)
    (if (Utilities|Enum|Equal(Enum) _array_element "cutting")
      (bind _returnvalue (Actor|GetActorOfClass "/Game/Blueprints/GameManagers/BP_CropManager.BP_CropManager_C"))
      (if (== (Variables|/Script/VCFarming.CropManager|Getcount _returnvalue) 0)
        (bind _returnvalue_2 (UserInterface|CreateWidget "/Game/Widgets/WBP_UtilityFarm1.WBP_UtilityFarm1_C"))
        (UserInterface|Viewport|AddtoViewport _returnvalue_2 0)
        (elif (== (Variables|/Script/VCFarming.CropManager|Getcount _returnvalue) 1)
          (bind _returnvalue_3 (UserInterface|CreateWidget "/Game/Widgets/WBP_UtilityFarm2.WBP_UtilityFarm2_C"))
          (UserInterface|Viewport|AddtoViewport _returnvalue_3 0)
          (elif (== (Variables|/Script/VCFarming.CropManager|Getcount _returnvalue) 2)
            (bind _returnvalue_4 (UserInterface|CreateWidget "/Game/Widgets/WBP_UtilityFarm3.WBP_UtilityFarm3_C"))
            (UserInterface|Viewport|AddtoViewport _returnvalue_4 0)
            (elif (== (Variables|/Script/VCFarming.CropManager|Getcount _returnvalue) 3)
              (bind _returnvalue_5 (UserInterface|CreateWidget "/Game/Widgets/WBP_UtilityFarm4.WBP_UtilityFarm4_C"))
              (UserInterface|Viewport|AddtoViewport _returnvalue_5 0)
              (elif (== (Variables|/Script/VCFarming.CropManager|Getcount _returnvalue) 4)
                (bind _returnvalue_6 (UserInterface|CreateWidget "/Game/Widgets/WBP_UtilityFarm5.WBP_UtilityFarm5_C"))
                (UserInterface|Viewport|AddtoViewport _returnvalue_6 0)))))))))

(event EventBeginPlay
  (EventDispatchers|BindEventtoOnWordsSpoken (Subsystems|GetSpeechRecognitionSubsystem) (delegate Custom|TriggerSpeech)))

(event Collision|EventActorBeginOverlap
  (params (OtherActor :type Actor%20Object%20Reference)))

(event EventTick
  (params (DeltaSeconds :type Float%20%28single-precision%29)))

(fn ConstructionScript)