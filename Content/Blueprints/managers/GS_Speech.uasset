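; GS_Speech is a manager Blueprint, likely a Game State by its prefix, that sets up voice keyword recognition for the game.
; On BeginPlay it puts the speech recognition subsystem into keyword mode with a phrase list covering farm selection, market and cutting commands, each with a match tolerance.
; On EndPlay it shuts the subsystem down.
; It does not handle recognized phrases itself.
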(event EventBeginPlay
  (Class|SpeechRecognitionSubsystem|EnableKeywordMode (Subsystems|GetSpeechRecognitionSubsystem) (Utilities|Array|MakeArray (Utilities|Struct|MakeRecognitionPhrase "farm one" "VE_7") (Utilities|Struct|MakeRecognitionPhrase "farm two" "VE_7") (Utilities|Struct|MakeRecognitionPhrase "farm three" "VE_7") (Utilities|Struct|MakeRecognitionPhrase "farm four" "VE_7") (Utilities|Struct|MakeRecognitionPhrase "farm five" "VE_7") (Utilities|Struct|MakeRecognitionPhrase "open market" "VE_7") (Utilities|Struct|MakeRecognitionPhrase "cutting" "VE_5") "" "" "" "" "" "" "" "" "" "" "" "" "" "" "" "" "" "" "" "" "" "" "" "" "")))

(event EventTick
  (params (DeltaSeconds :type Float%20%28single-precision%29)))

(event EventEndPlay
  (params (EndPlayReason :type EEndPlayReason%20Enum :default "Destroyed"))
  (Class|SpeechRecognitionSubsystem|Shutdown (Subsystems|GetSpeechRecognitionSubsystem)))

(fn ConstructionScript)